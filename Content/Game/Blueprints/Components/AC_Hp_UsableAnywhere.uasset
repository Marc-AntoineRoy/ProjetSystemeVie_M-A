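; Reusable health component that tracks an actor's current and maximum HP and death state.
; Damage and heal events are ignored while dead, whereas reset revives to full HP.
; All three events route through one update function that clamps HP, broadcasts an HP-changed dispatcher, and sets the dead flag, firing a death dispatcher when HP reaches zero.
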(event `/Game/Game/Blueprints/Interfaces/BPI_Damageable_UsableAnywhere.TakeDmg`
  (params (DgmTakenAmount :type "Float (double-precision)"))
  ; Take Dmg calcule
  (if (not (`self.isDead`))
    (`self.UpdateHpAndNotify` (- (`self.currentHp`) DgmTakenAmount))))

(event `/Game/Game/Blueprints/Interfaces/BPI_Damageable_UsableAnywhere.GainHp`
  (params (HpGainedAmount :type "Float (double-precision)"))
  ; Gain Hp calcule
  (if (not (`self.isDead`))
    (`self.UpdateHpAndNotify` (+ (`self.currentHp`) HpGainedAmount))))

(event `/Game/Game/Blueprints/Interfaces/BPI_Damageable_UsableAnywhere.ResetHp`
  ; Reset Hp calcule
  (set `self.isDead` false)
  (`self.UpdateHpAndNotify` (`self.maxHp`)))

(fn `UpdateHpAndNotify`
  (params (NewHpValue :type "Float (double-precision)"))
  (bind _maxhp (`self.maxHp`))
  ; Update les variable du AC_Hp, nous invoquons le OnHpChanged pour indiquer un changement du HP
  ; Call le OnDeath si Hp = 0
  (bind _output_get (set `self.currentHp` (`KismetMathLibrary.FClamp` NewHpValue 0.0 _maxhp)))
  (`self.OnHpChanged` _output_get _maxhp)
  (if (<= (`self.currentHp`) 0.0)
    (set `self.isDead` true)
    (`self.OnDeath`)
    (else
      (set `self.isDead` false))))