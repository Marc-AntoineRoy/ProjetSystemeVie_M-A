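; BP_HpPickup is a pickup actor that heals or damages the third-person player character on overlap.
; Its Collision begin-overlap reaches the ACHp component on the character's BP_PlayerState.
; The sign of HpChangeAmount selects TakeDmg or GainHp, and the DestroyActor flag decides whether the pickup then removes itself.
; End overlap only performs the casts and has no further effect.
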(event `self.Collision.OnComponentBeginOverlap`
  (params (OverlappedComponent :type "PrimitiveComponent Object Reference") (OtherActor :type "Actor Object Reference") (OtherComp :type "PrimitiveComponent Object Reference") (OtherBodyIndex :type Integer) (bFromSweep :type Boolean) (SweepResult :type "HitResult Structure (by ref)"))
  ; Overlapping
  ;; Start overlap
  (bind _asbp_third_person_character (cast `/Game/Game/Blueprints/Pawns_Characters/Player/BP_ThirdPersonCharacter` OtherActor))
  (bind _asbp_player_state (cast `/Game/Game/Blueprints/Pawns_Characters/Player/BP_PlayerState` (`Pawn.PlayerState` _asbp_third_person_character)))
  ;; hp change
  (if (< (`self.HpChangeAmount`) 0.0)
    (bind _ac_hp (`/Game/Game/Blueprints/Pawns_Characters/Player/BP_PlayerState.AC_Hp` _asbp_player_state))
    ;;; lose hp
    (`/Game/Game/Blueprints/Components/AC_Hp_UsableAnywhere.TakeDmg` _ac_hp (`KismetMathLibrary.Abs` (`self.HpChangeAmount`)))
    (else
      ;;; gain hp
      (`/Game/Game/Blueprints/Interfaces/BPI_Damageable_UsableAnywhere.GainHp` _ac_hp (`self.HpChangeAmount`))))
  ;; Destroy actor if true
  (if (`self.DestroyActor`)
    (`self.K2_DestroyActor`)))

(event `self.Collision.OnComponentEndOverlap`
  (params (OverlappedComponent :type "PrimitiveComponent Object Reference") (OtherActor :type "Actor Object Reference") (OtherComp :type "PrimitiveComponent Object Reference") (OtherBodyIndex :type Integer))
  ; En overlap
  (bind _asbp_third_person_character (cast `/Game/Game/Blueprints/Pawns_Characters/Player/BP_ThirdPersonCharacter` OtherActor))
  (cast `/Game/Game/Blueprints/Pawns_Characters/Player/BP_PlayerState` (`Pawn.PlayerState` _asbp_third_person_character)))

(fn `UserConstructionScript`)